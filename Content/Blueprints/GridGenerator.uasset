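; Grid generator actor that builds a tile board at play start and places a random race start and finish on it.
; After a short delay, nested loops spawn GridSlot actors at even spacing from its location into TileArray.
; Random indices, bounded by a minimum for the end and a maximum for the start, pick tiles to replace with race actors.
; Player pawn 1 moves just above the start, while pawn 0 matches its XY and keeps its height.
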(event EventBeginPlay
  (Utilities|FlowControl|Delay 0.2)
  (CallFunction|GenerateGrid)
  (CallFunction|GenerateRaceEnd)
  (CallFunction|GenerateRaceStart))

(event Collision|EventActorBeginOverlap
  (params (OtherActor :type Actor%20Object%20Reference)))

(event EventTick
  (params (DeltaSeconds :type Float%20%28single-precision%29)))

(fn ConstructionScript)

(fn GenerateGrid
  (LocalVariables|SetyLocalPos (Variables|GridGeneration|GettilePositionDifference))
  (for _index (range 1 (Variables|GridGeneration|GetsizeX))
    (bind _returnvalue (Game|SpawnActorfromClass "/Game/Blueprints/gridSlot.gridSlot_C" (Math|Transform|MakeTransform (+ (Transformation|GetActorLocation) (Math|Vector|MakeVector (LocalVariables|GetxLocalPos) 0.0 0.0)) "0, 0, 0" "1,1,1") "Undefined" 0 0))
    (Utilities|Array|Add (Variables|GridGeneration|GettileArray) _returnvalue)
    (for _index_2 (range 1 (- (Variables|GridGeneration|GetsizeY) 1))
      (bind _returnvalue_2 (Game|SpawnActorfromClass "/Game/Blueprints/gridSlot.gridSlot_C" (Math|Transform|MakeTransform (+ (Transformation|GetActorLocation) (Math|Vector|MakeVector (LocalVariables|GetxLocalPos) (LocalVariables|GetyLocalPos) 0.0)) "0, 0, 0" "1,1,1") "Undefined" 0 0))
      (LocalVariables|SetyLocalPos (+ (LocalVariables|GetyLocalPos) (Variables|GridGeneration|GettilePositionDifference)))
      (Utilities|Array|Add (Variables|GridGeneration|GettileArray) _returnvalue_2))
    (LocalVariables|SetxLocalPos (+ (LocalVariables|GetxLocalPos) (Variables|GridGeneration|GettilePositionDifference)))
    (LocalVariables|SetyLocalPos (Variables|GridGeneration|GettilePositionDifference))))

(fn GenerateRaceEnd
  (bind _output_get (LocalVariables|SetraceEndIndex (Math|Random|RandomIntegerinRange (Variables|GridGeneration|GetminimumEndGenerationIndex) (* (Variables|GridGeneration|GetsizeX) (Variables|GridGeneration|GetsizeY)))))
  (Game|SpawnActorfromClass (Variables|Default|GetraceEndActor) (Math|Transform|MakeTransform (.location (Transformation|GetActorTransform (Utilities|Array|Get(acopy) (Variables|GridGeneration|GettileArray) _output_get))) (.rotation (Transformation|GetActorTransform (Utilities|Array|Get(acopy) (Variables|GridGeneration|GettileArray) _output_get))) "1,1,1") "Undefined" 0 0)
  (Actor|DestroyActor (Utilities|Array|Get(acopy) (Variables|GridGeneration|GettileArray) _output_get)))

(fn GenerateRaceStart
  (bind _returnvalue (Game|Player|GetPlayerPawn 0))
  (bind _output_get (LocalVariables|SetraceIndex (Math|Random|RandomInteger (Variables|GridGeneration|GetmaximumStartGenerationIndex))))
  (bind _returnvalue_2 (Game|SpawnActorfromClass (Variables|Default|GetraceStartActor) (Math|Transform|MakeTransform (.location (Transformation|GetActorTransform (Utilities|Array|Get(acopy) (Variables|GridGeneration|GettileArray) _output_get))) (.rotation (Transformation|GetActorTransform (Utilities|Array|Get(acopy) (Variables|GridGeneration|GettileArray) _output_get))) "1,1,1") "Undefined" 0 0))
  (Actor|DestroyActor (Utilities|Array|Get(acopy) (Variables|GridGeneration|GettileArray) _output_get))
  (Transformation|SetActorLocation (Game|Player|GetPlayerPawn 1) (+ (.location (Transformation|GetActorTransform _returnvalue_2)) "0, 0,40.000000") false true)
  (Transformation|SetActorLocation _returnvalue (Math|Vector|MakeVector (.X (Math|Vector|BreakVector (.location (Transformation|GetActorTransform _returnvalue_2)))) (.Y (Math|Vector|BreakVector (.location (Transformation|GetActorTransform _returnvalue_2)))) (.z (Transformation|GetActorLocation _returnvalue))) false false))
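; Constructor is a camera actor for tile building, showing the cursor and edge-scrolling via local offsets.
; Mouse axis events drive the ScreenEdgeMovement macro, which compares cursor position with viewport edges, dividing both axes by viewport height.
; DetectGridSlot stores the actor under the cursor; Place replaces a slot with a spawned tile and flags GM's choice.
; Their event-graph calls are unwired, as are the camera-focus and movement helpers.
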(event EventBeginPlay
  (Variables|/Script/Engine.PlayerController|SetbShowMouseCursor (Game|GetPlayerController 0) true))

(event Collision|EventActorBeginOverlap
  (params (OtherActor :type Actor%20Object%20Reference)))

(event EventTick
  (params (DeltaSeconds :type Float%20%28single-precision%29)))

(event Input|MouseEvents|MouseX
  (params (AxisValue :type Float%20%28single-precision%29))
  (Utilities|ScreenEdgeMovement) ; enters at MouseY
)

(event Input|MouseEvents|MouseY
  (params (AxisValue :type Float%20%28single-precision%29))
  (bind (_deltaxspeed _deltayspeed) (Utilities|ScreenEdgeMovement)
    (:ReturnNode
      (Transformation|AddActorLocalOffset (Math|Vector|MakeVector _deltaxspeed _deltayspeed 0.0) false false))))

(event Input|MouseEvents|LeftMouseButton
  (params (Key :type Key%20Structure :default "None")))

(fn ConstructionScript)

(fn FocustoPlayer
  (Transformation|SetWorldRotation (Variables|Default|GetCamera) (Math|Rotator|FindLookatRotation (Transformation|GetActorLocation) (Transformation|GetActorLocation (Variables|Default|GetActorToFocus))) false false))

(fn Movement
  (Transformation|AddActorLocalOffset (* (Variables|Default|GetmovementVector) (Variables|Movement|Getspeed)) false false))

(fn DetectGridSlot
  (Variables|Default|SetNextSlot (.HitActor (Collision|BreakHitResult (.HitResult (Game|Player|GetHitResultUnderCursorbyChannel (Game|GetPlayerController 0) "TraceTypeQuery2" false))))))

(fn Place
  (params (TileToCreate :type Tile%20Base%20Class%20Reference) (slot :type Actor%20Object%20Reference))
  (Utilities|IsValid slot
    (:Is%20Valid
      (Game|SpawnActorfromClass TileToCreate (Math|Transform|MakeTransform (.location (Transformation|GetActorTransform slot)) "0, 0, 0" "1,1,1") "Undefined" 0 0 0)
      (Actor|DestroyActor slot)
      (Variables|/Game/Blueprints/GM.GM_C|SetConstructorHasChoose (.AsGM (Utilities|Casting|CastToGM (Game|GetGameMode))) true))))
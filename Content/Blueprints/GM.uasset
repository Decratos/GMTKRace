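; GM manages a two-player constructor race, ensuring a second local player and pointing the Constructor pawn's focus at the other pawn.
; It creates the ConstructorUI, which displays a minutes/seconds race countdown updated on Tick until someone finishes.
; After the constructor chooses, a delay timer refreshes the random tile offer, rolling stored tiles and displayed icons separately.
; The time-up message is only a debug print, unreachable as wired.
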(event EventBeginPlay
  (bind _returnvalue (Class|GameModeBase|GetNumPlayers))
  (if (< _returnvalue 2)
    (Class|GameplayStatics|CreatePlayer -1))
  (Variables|Default|SetPlayer1 (Game|Player|GetPlayerPawn 0))
  (bind _output_get (Variables|Default|SetPlayer2 (Game|Player|GetPlayerPawn 1)))
  (Variables|/Game/Blueprints/Constructor.Constructor_C|SetActorToFocus (.AsConstructor (Utilities|Casting|CastToConstructor (Variables|Default|GetPlayer1))) _output_get)
  (bind _returnvalue_2 (UserInterface|CreateWidget "/Game/Blueprints/Widget/ConstructorUI.ConstructorUI_C" (Class|GameplayStatics|GetPlayerControllerfromID)))
  (UserInterface|Viewport|AddtoViewport _returnvalue_2 0)
  (Variables|Default|SetConstructorWidget _returnvalue_2)
  (Variables|Default|SetactualMinutesRemaining (Variables|Default|Getminutes))
  (Variables|Default|SetactualSecondsRemaining (Variables|Default|Getseconds)))

(event EventTick
  (params (DeltaSeconds :type Float%20%28single-precision%29))
  (CallFunction|TimerManaging)
  (CallFunction|RaceTimeManager))

(fn ConstructionScript)

(fn TimerManaging
  (if (Variables|TileGeneration|GetConstructorHasChoose)
    (bind _output_get (Variables|TileGeneration|SetactualTimeBetweenNewTiles (- (Variables|TileGeneration|GetactualTimeBetweenNewTiles) (* 1.0 (Utilities|Time|GetWorldDeltaSeconds)))))
    (if (<= _output_get 0.0)
      (CallFunction|GenerateNewTiles))))

(fn GenerateNewTiles
  (bind _tileslist (Variables|TileGeneration|GettilesList))
  (bind _tileslist_2 (Variables|TileGeneration|GettilesList))
  (bind _returnvalue (Utilities|Array|Length _tileslist_2))
  (bind _returnvalue_2 (- _returnvalue 1))
  (bind _returnvalue_3 (Math|Random|RandomIntegerinRange 0 _returnvalue_2))
  (bind _output (Utilities|Array|Get(acopy) _tileslist _returnvalue_3))
  (Utilities|Array|Clear (Variables|TileGeneration|GetRandomlyChooseTile))
  (Variables|TileGeneration|SetConstructorHasChoose false)
  (Variables|TileGeneration|SetactualTimeBetweenNewTiles (Math|Conversions|ToFloat(Integer) (Variables|TileGeneration|GettimeBetweenNewTiles)))
  (Default|ClearTilesIconList (Variables|Default|GetConstructorWidget))
  (for _index (range 1 (Variables|TileGeneration|GetnumberOfTileGiven))
    (Utilities|Array|Add (Variables|TileGeneration|GetRandomlyChooseTile) _output)
    (Default|GenerateTileIcon (Variables|Default|GetConstructorWidget) _output)))

(fn RaceTimeManager
  (if (not (Variables|Default|GetplayerHasFinishedTheRace))
    (bind _output_get (Variables|Default|SetactualSecondsRemaining (- (Variables|Default|GetactualSecondsRemaining) (* 1.0 (Utilities|Time|GetWorldDeltaSeconds)))))
    (if (<= _output_get 0.0)
      (if (> (Variables|Default|GetactualMinutesRemaining) 0)
        (bind _output_get_2 (Variables|Default|SetactualMinutesRemaining (- (Variables|Default|GetactualMinutesRemaining) 1)))
        (Variables|Default|SetactualSecondsRemaining 6e+01)
        (Default|SetTimeText (Variables|Default|GetConstructorWidget) _output_get_2 (Math|Float|Truncate (Variables|Default|GetactualSecondsRemaining)) :!label _label)
        (if (and (<= (Variables|Default|GetactualMinutesRemaining) 0) (<= (Variables|Default|GetactualSecondsRemaining) 0.0))
          (Development|PrintString "Fin du temps")))
      (else
        (goto _label)))))